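; BP_Showcase is a showcase actor that displays a skeletal mesh on an optional platform, with a rotating spring-arm camera.
; BeginPlay creates a hidden ShowcaseHUD, and the ActivarInput action toggles its visibility and input mode.
; Events set camera speed, model speed and platform visibility, which Tick applies as frame-rate-dependent yaw centred on 0.5 and as visibility.
; Tick also forces the cursor visible, overriding DisableMouse.
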(event `self.ReceiveBeginPlay`
  ;[1 1 1] Set HUD
  (bind _returnvalue (`|CreateWidget` "/Game/Showcase/UMG/ShowcaseHUD.ShowcaseHUD_C"))
  (bind _output_get (set `self.ShowcaseHudReference` _returnvalue))
  (`UserWidget.AddToViewport` _output_get 0)
  (`Widget.SetVisibility` _output_get "Hidden"))

(event `self.ReceiveTick`
  (params (DeltaSeconds :type "Float (single-precision)"))
  ;[1 1 1] Camera Rotation
  (set `PlayerController.bShowMouseCursor` true (`GameplayStatics.GetPlayerController` 0))
  (`SceneComponent.K2_AddLocalRotation` (`self.SpringArm`) (`KismetMathLibrary.MakeRotator` 0.0 0.0 (* (- (`self.SpeedCamera`) 0.5) 0.4)) false false)
  ;[1 1 1] Mesh Rotation
  (`SceneComponent.K2_AddLocalRotation` (`self.SkeletalMesh`) (`KismetMathLibrary.MakeRotator` 0.0 0.0 (* (- (`self.SpeedModel`) 0.5) 0.4)) false false)
  (`SceneComponent.SetVisibility` (`self.Platform`) (`self.IsPlatformVisible?`) false))

(event `InputAction|ActivarInput`
  (params (Key :type "Key Structure" :default "AnyKey"))
  (bind _showcasehudreference (`self.ShowcaseHudReference`))
  ;[1 1 1] Enable/Disable Mouse Controls
  (:`Pressed`
    (`/Engine/EditorBlueprintResources/StandardMacros.FlipFlop`
      (:`A`
        (`Widget.SetVisibility` _showcasehudreference "Visible")
        (`self.EnableMouse`))
      (:`B`
        (`Widget.SetVisibility` _showcasehudreference "Hidden")
        (`self.DisableMouse`)))))

(event `/Game/Showcase/ShowcaseInterface.ChangeSpeedCamera`
  (params (Speed :type "Float (single-precision)"))
  ;[1 1 1] Change Speed Camera
  (set `self.SpeedCamera` Speed))

(event `/Game/Showcase/ShowcaseInterface.ChangeSpeedModel`
  (params (Speed :type "Float (single-precision)"))
  ;[1 1 1] Change Speed Model
  (set `self.SpeedModel` Speed))

(event `/Game/Showcase/ShowcaseInterface.ChangePlatformVisibility`
  (params (`IsVisible?` :type Boolean))
  (set `self.IsPlatformVisible?` `IsVisible?`))

(fn `DisableMouse`
  (`WidgetBlueprintLibrary.SetInputMode_GameOnly` null)
  (set `PlayerController.bShowMouseCursor` false (`GameplayStatics.GetPlayerController` 0)))

(fn `EnableMouse`
  (bind _returnvalue (`GameplayStatics.GetPlayerController` 0))
  (`WidgetBlueprintLibrary.SetInputMode_GameAndUIEx` _returnvalue (`self.ShowcaseHudReference`))
  (set `PlayerController.bShowMouseCursor` true _returnvalue))

(fn `UserConstructionScript`)